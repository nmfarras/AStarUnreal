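; BP_Item is an axis-input-driven actor that keeps requesting a path from itself to a BP_target actor.
; BeginPlay finds the level's first CameraActor, blends the player's view to it with a fixed FOV, and caches the target and a Pathfinder actor.
; Tick calls FindPath toward the target, re-fetching it if missing, while MoveRight and MoveUp shift the actor along world Y and X.
; Zoom and timer logic are disconnected.
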(event Custom|finder)

(event EventBeginPlay
  (Utilities|FlowControl|Sequence
    (:then_0
      (bind _outactors (Actor|GetAllActorsOfClass "/Script/Engine.CameraActor"))
      (Variables|Default|SetCamera (Utilities|Array|Get(acopy) _outactors))
      (Game|Player|SetViewTargetwithBlend (Game|GetPlayerController 0) (Utilities|Array|Get(acopy) _outactors) 0.0 "VTBlend_Linear" 0.0 false))
    (:then_1
      (bind _outactors_2 (Actor|GetAllActorsOfClass "/Game/BP_target.BP_target_C"))
      (Variables|Default|SetTarget (Utilities|Array|Get(acopy) _outactors_2)))
    (:then_2
      (bind _outactors_3 (Actor|GetAllActorsOfClass "/Script/RacingGame.Pathfinder"))
      (Variables|Default|SetPath (Utilities|Array|Get(acopy) _outactors_3)))
    (:then_3
      (Camera|SetFieldOfView (Variables|/Script/Engine.CameraActor|GetCameraComponent (Variables|Default|GetCamera)) 9e+01))))

(event EventTick
  (params (DeltaSeconds :type Float%20%28single-precision%29))
  (if (!= (Variables|Default|GetTarget) 0)
    (Class|Pathfinder|FindPath (Variables|Default|GetPath) (Transformation|GetActorLocation) (Transformation|GetActorLocation (Variables|Default|GetTarget)))
    (else
      (bind _outactors (Actor|GetAllActorsOfClass "/Game/BP_target.BP_target_C"))
      (Variables|Default|SetTarget (Utilities|Array|Get(acopy) _outactors)))))

(event Input|AxisEvents|InputAxisZoom
  (params (AxisValue :type Float%20%28single-precision%29)))

(event Input|AxisEvents|InputAxisMoveRight
  (params (AxisValue :type Float%20%28single-precision%29))
  (bind _returnvalue (Transformation|GetActorLocation))
  (Transformation|SetActorLocation (Math|Vector|MakeVector (.x _returnvalue) (.y (+ (Math|Vector|MakeVector 0.0 (.y _returnvalue) 0.0) (* AxisValue (Variables|Default|Getspeed)))) (.z _returnvalue)) false false))

(event Input|AxisEvents|InputAxisMoveUp
  (params (AxisValue :type Float%20%28single-precision%29))
  (bind _returnvalue (Transformation|GetActorLocation))
  (Transformation|SetActorLocation (Math|Vector|MakeVector (.x (+ (Math|Vector|MakeVector (.x _returnvalue) 0.0 0.0) (* AxisValue (Variables|Default|Getspeed)))) (.y _returnvalue) (.z _returnvalue)) false false))

(fn ConstructionScript)